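; BP_Door is a swinging door prop that shows a UI widget while the player is nearby.
; Each OpenDoor call alternates through a FlipFlop between playing and reversing a timeline that lerps Door1's relative yaw to swing it open or closed.
; A WB_Door widget, created on BeginPlay, is added to the viewport when the player character enters UI_Box and removed on exit.
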(event OnComponentBeginOverlap(UI_Box)
  (params (OverlappedComponent :type Primitive%20Component%20Object%20Reference) (OtherActor :type Actor%20Object%20Reference) (OtherComp :type Primitive%20Component%20Object%20Reference) (OtherBodyIndex :type Integer) (bFromSweep :type Boolean) (SweepResult :type Hit%20Result%20Structure%20%28by%20ref%29))
  (if (== OtherActor (Game|GetPlayerCharacter 0))
    (UserInterface|Viewport|AddtoViewport (Variables|Default|GetUI) 0)))

(event OnComponentEndOverlap(UI_Box)
  (params (OverlappedComponent :type Primitive%20Component%20Object%20Reference) (OtherActor :type Actor%20Object%20Reference) (OtherComp :type Primitive%20Component%20Object%20Reference) (OtherBodyIndex :type Integer))
  (if (== OtherActor (Game|GetPlayerCharacter 0))
    (Widget|RemovefromParent (Variables|Default|GetUI))))

(event Custom|OpenDoor
  (Utilities|FlowControl|FlipFlop
    (:A
      (bind _door (Timeline|OpenDoorTimeLine PlayFromStart)
        (:Update
          (Transformation|SetRelativeRotation (Variables|Default|GetDoor1) (Math|Rotator|MakeRotator 0.0 0.0 (Math|Float|Lerp 0.0 9e+01 _door)) false false))))
    (:B
      (Timeline|OpenDoorTimeLine Reverse))))

(event EventBeginPlay
  (bind _returnvalue (UserInterface|CreateWidget "/Game/UI/WB_Door.WB_Door_C"))
  (Variables|Default|SetUI _returnvalue))

(fn ConstructionScript)